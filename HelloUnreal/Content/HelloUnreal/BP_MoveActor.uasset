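; Practice actor in HelloUnreal that moves its static mesh in a rising staircase pattern.
; Tick adds a fixed step each frame, not scaled by delta time, to the relative X or Z location, using a distance counter to flip IsMoveRight between longer horizontal and shorter vertical runs.
; BeginPlay prints a string-split test.
; Disconnected nodes hold earlier movement, print and string-function experiments that never run.
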(event EventTick
  (params (DeltaSeconds :type Float%20%28single-precision%29))
  ;[0.15 0.15 0.15 0.5] 계단식으로 움직이기(LocationCheck 값을 만들어서 저장하고 그 값이 원하는 만큼의 이동을 넘었을 때 Check 값을 초기화 하고 다른 쪽으로 이동하게 변경)
  (if (Variables|Default|GetIsMoveRight)
    ;;[0.15 0.15 0.15 0.5] 오른쪽으로 상자 움직이기
    ;;;[0.15 0.15 0.15 0.5] LocationX에 1을 더한 값을 LocationX에 넣는다
    (Variables|Default|SetLocationX (+ (Variables|Default|GetLocationX) 1.0))
    (Variables|Default|SetLocationCheck (+ (Variables|Default|GetLocationCheck) 1.0))
    ;;;[0.15 0.15 0.15 0.5] 상대 좌표를 설정
    (Transformation|SetRelativeLocation (Variables|Default|GetStaticMesh) (Math|Vector|MakeVector (Variables|Default|GetLocationX) 0.0 (Variables|Default|GetLocationZ)) false false)
    ;;[0.15 0.15 0.15 0.5] Check 값 확인
    (if (> (Variables|Default|GetLocationCheck) 1e+02)
      ;;[0.15 0.15 0.15 0.5] Check 값 초기화, IsMoveRight 값 변경
      (Variables|Default|SetLocationCheck 0.0)
      (Variables|Default|SetIsMoveRight false))
    (else
      ;;[0.15 0.15 0.15 0.5] 위쪽으로 상자 움직이기
      ;;;[0.15 0.15 0.15 0.5] LocationZ에 1을 더한 값을 LocationZ에 넣는다
      (Variables|Default|SetLocationZ (+ (Variables|Default|GetLocationZ) 1.0))
      (Variables|Default|SetLocationCheck (+ (Variables|Default|GetLocationCheck) 1.0))
      ;;;[0.15 0.15 0.15 0.5] 상대 좌표를 설정
      (Transformation|SetRelativeLocation (Variables|Default|GetStaticMesh) (Math|Vector|MakeVector (Variables|Default|GetLocationX) 0.0 (Variables|Default|GetLocationZ)) false false)
      ;;[0.15 0.15 0.15 0.5] Check 값 확인
      (if (> (Variables|Default|GetLocationCheck) 5e+01)
        ;;[0.15 0.15 0.15 0.5] Check 값 초기화, IsMoveRight 값 변경
        (Variables|Default|SetLocationCheck 0.0)
        (Variables|Default|SetIsMoveRight true)))))

(event EventBeginPlay
  (bind _returnvalue (Utilities|String|MakeLiteralString "abc,def,ghi.asid"))
  (bind (_lefts _rights _returnvalue_2) (Utilities|String|Split _returnvalue ","))
  (Development|PrintString (Utilities|String|Append _lefts "/" _rights (Utilities|String|ToString(Boolean) _returnvalue_2)) true true "(R=0.000000,G=0.660000,B=1.000000,A=1.000000)" 3e+01))

(fn ConstructionScript)